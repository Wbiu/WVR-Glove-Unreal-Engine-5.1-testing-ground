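; Serial COM bridge to a hand-tracking device with per-finger force feedback, apparently a haptic glove.
; BeginSerialComConnection opens the port; Deserializer passes each read string to SplitDataSet, which parses a brace-wrapped, semicolon-delimited packet into clamped finger positions and gyro rotation.
; SendFFB latches each finger's hit state and writes combined force values only on change, while ReleaseFFB sends the no-force string.
; Location parsing and tolerance filtering are disconnected.
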(event `/Game/SerialCOM/SerialCOM_BP_Interface.Close Connection`
  (bind _my_serial (`self.My Serial`))
  ;[1 1 1] Closing Serial COM
  (`/Engine/EditorBlueprintResources/StandardMacros.IsValid` _my_serial
    (:`Is Valid`
      (`SerialCom.Close` _my_serial))))

(event `/Game/SerialCOM/SerialCOM_BP_Interface.Deserializer`
  ;[1 1 1] Deserialze Data Reciev
  (bind (_bsuccess _returnvalue) (`SerialCom.ReadString` (`self.My Serial`)))
  (`self.Split Data Set` _returnvalue))

(fn `Begin Serial Com Connection`
  (bind (_bopened _returnvalue) (`SerialCom.OpenComPortWithFlowControl` (`self.Port`) (`self.Bound Rate`)))
  (if (`SerialCom.IsOpened` _returnvalue)
    (bind _output_get (set `self.My Serial` _returnvalue))
    (`SerialCom.Flush` _output_get)
    (`KismetSystemLibrary.PrintString` "Serial Connected")
    (else
      (`KismetSystemLibrary.PrintString` "Serial COM not Connected !" true true (struct :`R` 1.0 :`G` 0.044498 :`A` 1.0)))))

(fn `Release FFB`
  (locals (noFFB :type String :default "0;0;0;0;0\\0"))
  (`SerialCom.Println` (`self.My Serial`) (`local.noFFB`))
  (set `self.setFFB_Thm_once` false)
  (set `self.setFFB_Idx_once` false))

(fn `Send FFB`
  (params (thmb_ffb :type Boolean) (stillHitThb :type Boolean) (idx_ffb :type Boolean) (stillHitIdx :type Boolean) (mdl_ffb :type Boolean) (stillHitMdl :type Boolean) (rng_ffb :type Boolean) (StillHitRing :type Boolean) (pky_ffb :type Boolean) (StillHitPky :type Boolean))
  (bind _seperator (`self.Seperator`))
  (bind _returnvalue (`KismetStringLibrary.Concat_StrStr` (`KismetStringLibrary.Conv_IntToString` (`self.FFBValThb`)) _seperator (`KismetStringLibrary.Conv_IntToString` (`self.FFBValIdx`)) _seperator (`KismetStringLibrary.Conv_IntToString` (`self.FFBValMdl`)) _seperator (`KismetStringLibrary.Conv_IntToString` (`self.FFBValRng`)) _seperator (`KismetStringLibrary.Conv_IntToString` (`self.FFBValPky`))))
  (`|ExecutionSequence`
    (:`then_0`
      (if thmb_ffb
        (if stillHitThb
          (if (not (`self.setFFB_Thm_once`))
            (set `self.FFBValThb` (`self.defaultFFBForce`))
            (set `self.setFFB_Thm_once` true)
            (set `self.isFFB_Val_changed` true :!label _label)))
        (elif (`self.setFFB_Thm_once`)
          (set `self.FFBValThb` 0)
          (set `self.setFFB_Thm_once` false)
          (goto _label))))
    (:`then_1`
      (if idx_ffb
        (if stillHitIdx
          (if (not (`self.setFFB_Idx_once`))
            (set `self.FFBValIdx` (`self.defaultFFBForce`))
            (set `self.setFFB_Idx_once` true)
            (set `self.isFFB_Val_changed` true :!label _label_2)))
        (elif (`self.setFFB_Idx_once`)
          (set `self.FFBValIdx` 0)
          (set `self.setFFB_Idx_once` false)
          (goto _label_2))))
    (:`then_2`
      (if mdl_ffb
        (if stillHitMdl
          (if (not (`self.setFFB_Mdl_Once`))
            (set `self.FFBValMdl` (`self.defaultFFBForce`))
            (set `self.setFFB_Mdl_Once` true)
            (set `self.isFFB_Val_changed` true :!label _label_3)))
        (elif (`self.setFFB_Mdl_Once`)
          (set `self.FFBValMdl` 0)
          (set `self.setFFB_Mdl_Once` false)
          (goto _label_3))))
    (:`then_3`
      (if rng_ffb
        (if StillHitRing
          (if (not (`self.setFFB_Rng_Once`))
            (set `self.FFBValRng` (`self.defaultFFBForce`))
            (set `self.setFFB_Rng_Once` true)
            (set `self.isFFB_Val_changed` true :!label _label_4)))
        (elif (`self.setFFB_Rng_Once`)
          (set `self.FFBValRng` 0)
          (set `self.setFFB_Rng_Once` false)
          (goto _label_4))))
    (:`then_4`
      (if pky_ffb
        (if StillHitPky
          (if (not (`self.setFFB_Pky_Once`))
            (set `self.FFBValPky` (`self.defaultFFBForce`))
            (set `self.setFFB_Pky_Once` true)
            (set `self.isFFB_Val_changed` true :!label _label_5)))
        (elif (`self.setFFB_Pky_Once`)
          (set `self.FFBValPky` 0)
          (set `self.setFFB_Pky_Once` false)
          (goto _label_5))))
    (:`then_5`
      (if (`self.isFFB_Val_changed`)
        (`KismetSystemLibrary.PrintString` _returnvalue)
        (`SerialCom.Println` (`self.My Serial`) _returnvalue)
        (set `self.isFFB_Val_changed` false)))))

(fn `Split Data Set`
  (params (`Data set` :type String))
  (bind _returnvalue (`KismetStringLibrary.ParseIntoArray` (`KismetStringLibrary.Split` (`.RightS` (`KismetStringLibrary.Split` `Data set` "{")) "}" "IgnoreCase" "FromEnd") ";" false))
  ;[1 1 1] Data splitting
  (if (and (`KismetArrayLibrary.Array_IsValidIndex` _returnvalue) (`KismetArrayLibrary.Array_IsValidIndex` _returnvalue 1) (`KismetArrayLibrary.Array_IsValidIndex` _returnvalue 2) (`KismetArrayLibrary.Array_IsValidIndex` _returnvalue 3) (`KismetArrayLibrary.Array_IsValidIndex` _returnvalue 4) (`KismetArrayLibrary.Array_IsValidIndex` _returnvalue 5) (`KismetArrayLibrary.Array_IsValidIndex` _returnvalue 6) (`KismetArrayLibrary.Array_IsValidIndex` _returnvalue 7) (`KismetArrayLibrary.Array_IsValidIndex` _returnvalue 8) (`KismetArrayLibrary.Array_IsValidIndex` _returnvalue 9) (`KismetArrayLibrary.Array_IsValidIndex` _returnvalue 10))
    (set `self.ThumbPos` (`KismetMathLibrary.MapRangeClamped` (`KismetStringLibrary.Conv_StringToDouble` (`|GetArrayItem` _returnvalue)) 0.0 109.0 0.0 91.790561))
    (set `self.IndexPos` (`KismetMathLibrary.MapRangeClamped` (`KismetStringLibrary.Conv_StringToDouble` (`|GetArrayItem` _returnvalue 1)) 0.0 137.0 0.0 56.0))
    (set `self.MiddlePos` (`KismetMathLibrary.MapRangeClamped` (`KismetStringLibrary.Conv_StringToDouble` (`|GetArrayItem` _returnvalue 2)) 0.0 97.0 0.0 68.0))
    (set `self.RingPos` (`KismetMathLibrary.MapRangeClamped` (`KismetStringLibrary.Conv_StringToDouble` (`|GetArrayItem` _returnvalue 3)) 0.0 83.0 0.0 71.0))
    (set `self.PinkyPos` (`KismetMathLibrary.MapRangeClamped` (`KismetStringLibrary.Conv_StringToDouble` (`|GetArrayItem` _returnvalue 4)) 0.0 94.0 0.0 79.0))
    (set `self.rotate_Gyro` (`KismetMathLibrary.MakeRotator` (`KismetStringLibrary.Conv_StringToDouble` (`|GetArrayItem` _returnvalue 6)) (* (`KismetStringLibrary.Conv_StringToDouble` (`|GetArrayItem` _returnvalue 7)) -1.0) (`KismetStringLibrary.Conv_StringToDouble` (`|GetArrayItem` _returnvalue 5))))))

(fn `UserConstructionScript`)

(fn `valueChangeTolarance`
  (params (Value :type "Float (double-precision)") (Error :type "Float (double-precision)") (toCompare :type "Float (double-precision)"))
  (returns (isWithin :type Boolean))
  (return (or (>= (- Value Error) toCompare) (<= (+ Error Value) toCompare))))