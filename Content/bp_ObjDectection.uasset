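; Detects finger contact for a VR hand and handles grabbing and picking up objects, as functions with no event logic.
; Line traces from five finger arrows flag zero-distance hits and store finger values, clearing when values drop below them.
; GrabbingMechanism freezes values of touching fingers.
; PickUpMechanism attaches the thumb-hit actor to VRHand on thumb-plus-finger contact, detaching when thumb or index contact is lost.
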(event `self.ReceiveBeginPlay`)

(fn `Grabbing Mechanism`
  (params (FingerDataSet :type "/Game/FingerDataSet Structure"))
  (returns (FingerDataSetOut :type "/Game/FingerDataSet Structure"))
  (`|ExecutionSequence`
    (:`then_0`
      (if (not (`self.isHit_thumb`))
        (bind _output_get (set `self.thm_buff` FingerDataSet_ThunbVal_6_7CF1BB4A4EB8A181C7190AAB48CF3D06))))
    (:`then_1`
      (if (not (`self.isHit_index`))
        (bind _output_get_2 (set `self.idx_buff` FingerDataSet_IndexVal_7_AD0F51B449DC632CF2490EB6ED9580C1))))
    (:`then_2`
      (if (not (`self.isHit_middle`))
        (bind _output_get_3 (set `self.mdl_buff` FingerDataSet_MiddleVal_8_B35064AA4E65CB1DC53330B83E9D8FE5))))
    (:`then_3`
      (if (not (`self.isHit_ring`))
        (bind _output_get_4 (set `self.rng_buff` FingerDataSet_RingVal_9_5CAFEBE84D4F73E998F5C4896FF11B61))))
    (:`then_4`
      (if (not (`self.IsHit_pinky`))
        (bind _output_get_5 (set `self.pky_buff` FingerDataSet_PinkyVal_10_CDA7C8E04655CAE7863064A61912EB0A))))
    (:`then_5`
      (return (make `/Game/FingerDataSet` _output_get _output_get_2 _output_get_3 _output_get_4 _output_get_5)))))

(fn `Object Detection`
  (params (FingerDataArrow :type "/Game/fingerDataArrow Structure"))
  (returns (FingerDataSet :type "/Game/FingerDataSet Structure") (`Hited Actor` :type "Actor Object Reference"))
  (bind _returnvalue (`SceneComponent.K2_GetComponentLocation` FingerDataArrow_pinkyArrow_25_0F64A73D42E03942A03ABAB476D66DDE))
  (bind _returnvalue_2 (`SceneComponent.K2_GetComponentLocation` FingerDataArrow_indexArrow_22_180F2A7A4C0D7672928128ADAB30CDF2))
  (bind _returnvalue_3 (`SceneComponent.K2_GetComponentLocation` FingerDataArrow_middleArrow_23_8D83A3384ECAD043A763FAB0EF8815E3))
  (bind _returnvalue_4 (`SceneComponent.K2_GetComponentLocation` FingerDataArrow_ringArrow_24_A2D29F704FC850AC8B72AE963CF7B584))
  (bind _returnvalue_5 (`SceneComponent.K2_GetComponentLocation` FingerDataArrow_thumbArrow_21_E95276374674EA5EB0A824BB71C4032A))
  (bind _returnvalue_6 (* (`KismetMathLibrary.Conv_RotatorToVector` (`SceneComponent.K2_GetComponentRotation` FingerDataArrow_thumbArrow_21_E95276374674EA5EB0A824BB71C4032A)) 10000))
  (bind _returnvalue_7 (* (`KismetMathLibrary.Conv_RotatorToVector` (`SceneComponent.K2_GetComponentRotation` FingerDataArrow_indexArrow_22_180F2A7A4C0D7672928128ADAB30CDF2)) 10000))
  (bind _returnvalue_8 (* (`KismetMathLibrary.Conv_RotatorToVector` (`SceneComponent.K2_GetComponentRotation` FingerDataArrow_middleArrow_23_8D83A3384ECAD043A763FAB0EF8815E3)) 10000))
  (bind _returnvalue_9 (* (`KismetMathLibrary.Conv_RotatorToVector` (`SceneComponent.K2_GetComponentRotation` FingerDataArrow_pinkyArrow_25_0F64A73D42E03942A03ABAB476D66DDE)) 10000))
  (bind _returnvalue_10 (* (`KismetMathLibrary.Conv_RotatorToVector` (`SceneComponent.K2_GetComponentRotation` FingerDataArrow_ringArrow_24_A2D29F704FC850AC8B72AE963CF7B584)) 10000))
  (`KismetSystemLibrary.DrawDebugLine` _returnvalue_5 _returnvalue_6)
  (bind _outhit (`KismetSystemLibrary.LineTraceSingleForObjects` _returnvalue_5 _returnvalue_6 (`|MakeArray` "ObjectTypeQuery2" :!type "EObjectTypeQuery Enum")))
  (if (`self.isHit_thumb`)
    (if (< FingerDataArrow_thumbVal_6_851082834DE9C41EEC4ECCB147E41B9F (`self.thumb_hit_position`))
      (set `self.isHit_thumb` false))
    (else
      (bind (_bblockinghit _binitialoverlap _time _distance _location _impactpoint _normal _impactnormal _physmat _hitactor _hitcomponent) (`GameplayStatics.BreakHitResult` _outhit))
      (if _bblockinghit
        (if (== (`KismetMathLibrary.Round` _distance) 0)
          (set `self.Hit Actor on thumb` _hitactor)
          (set `self.Hit Component on thunb` _hitcomponent)
          (set `self.IsPhysicsON` (`SceneComponent.IsSimulatingPhysics` _hitcomponent "None"))
          (set `self.thumb_hit_position` FingerDataArrow_thumbVal_6_851082834DE9C41EEC4ECCB147E41B9F)
          (set `self.isHit_thumb` true)
          (else
            (set `self.isHit_thumb` false))))))
  (`KismetSystemLibrary.DrawDebugLine` _returnvalue_2 _returnvalue_7)
  (bind _outhit_2 (`KismetSystemLibrary.LineTraceSingleForObjects` _returnvalue_2 _returnvalue_7 (`|MakeArray` "ObjectTypeQuery2" :!type "EObjectTypeQuery Enum")))
  (if (`self.isHit_index`)
    (if (< FingerDataArrow_indexVal_7_E86F850E4C98DDAE5D91C58FF30FBF57 (`self.index_hit_position`))
      (set `self.isHit_index` false))
    (else
      (bind (_bblockinghit_2 _binitialoverlap_2 _time_2 _distance_2) (`GameplayStatics.BreakHitResult` _outhit_2))
      (if _bblockinghit_2
        (if (== (`KismetMathLibrary.Round` _distance_2) 0)
          (set `self.index_hit_position` FingerDataArrow_indexVal_7_E86F850E4C98DDAE5D91C58FF30FBF57)
          (set `self.isHit_index` true)
          (else
            (set `self.isHit_index` false))))))
  (`KismetSystemLibrary.DrawDebugLine` _returnvalue_3 _returnvalue_8)
  (bind _outhit_3 (`KismetSystemLibrary.LineTraceSingleForObjects` _returnvalue_3 _returnvalue_8 (`|MakeArray` "ObjectTypeQuery2" :!type "EObjectTypeQuery Enum")))
  (if (`self.isHit_middle`)
    (if (< FingerDataArrow_middleVal_8_DA58550F4A75A9CE741B059686597D8A (`self.middle_hit_position`))
      (set `self.isHit_middle` false))
    (else
      (bind (_bblockinghit_3 _binitialoverlap_3 _time_3 _distance_3) (`GameplayStatics.BreakHitResult` _outhit_3))
      (if _bblockinghit_3
        (if (== (`KismetMathLibrary.Round` _distance_3) 0)
          (set `self.middle_hit_position` FingerDataArrow_middleVal_8_DA58550F4A75A9CE741B059686597D8A)
          (set `self.isHit_middle` true)
          (else
            (set `self.isHit_middle` false))))))
  (`KismetSystemLibrary.DrawDebugLine` _returnvalue_4 _returnvalue_10)
  (bind _outhit_4 (`KismetSystemLibrary.LineTraceSingleForObjects` _returnvalue_4 _returnvalue_10 (`|MakeArray` "ObjectTypeQuery2" :!type "EObjectTypeQuery Enum")))
  (if (`self.isHit_ring`)
    (if (< FingerDataArrow_ringVal_9_845B976B4BF202FC8089CABA330311A4 (`self.ring_hit_position`))
      (set `self.isHit_ring` false))
    (else
      (bind (_bblockinghit_4 _binitialoverlap_4 _time_4 _distance_4) (`GameplayStatics.BreakHitResult` _outhit_4))
      (if _bblockinghit_4
        (if (== (`KismetMathLibrary.Round` _distance_4) 0)
          (set `self.ring_hit_position` FingerDataArrow_ringVal_9_845B976B4BF202FC8089CABA330311A4)
          (set `self.isHit_ring` true)
          (else
            (set `self.isHit_ring` false))))))
  (`KismetSystemLibrary.DrawDebugLine` _returnvalue _returnvalue_9)
  (bind _outhit_5 (`KismetSystemLibrary.LineTraceSingleForObjects` _returnvalue _returnvalue_9 (`|MakeArray` "ObjectTypeQuery2" :!type "EObjectTypeQuery Enum")))
  (if (`self.IsHit_pinky`)
    (if (< FingerDataArrow_pinkyVal_10_321ABFD74A5C7F0B29D73EA22A9E7B87 (`self.Pinky hit position`))
      (set `self.IsHit_pinky` false))
    (else
      (bind (_bblockinghit_5 _binitialoverlap_5 _time_5 _distance_5) (`GameplayStatics.BreakHitResult` _outhit_5))
      (if _bblockinghit_5
        (if (== (`KismetMathLibrary.Round` _distance_5) 0)
          (set `self.Pinky hit position` FingerDataArrow_pinkyVal_10_321ABFD74A5C7F0B29D73EA22A9E7B87)
          (set `self.IsHit_pinky` true)
          (else
            (set `self.IsHit_pinky` false))))))
  (return (make `/Game/FingerDataSet` FingerDataArrow_thumbVal_6_851082834DE9C41EEC4ECCB147E41B9F FingerDataArrow_indexVal_7_E86F850E4C98DDAE5D91C58FF30FBF57 FingerDataArrow_middleVal_8_DA58550F4A75A9CE741B059686597D8A FingerDataArrow_ringVal_9_845B976B4BF202FC8089CABA330311A4 FingerDataArrow_pinkyVal_10_321ABFD74A5C7F0B29D73EA22A9E7B87) (`self.Hit Actor on thumb`)))

(fn `Pass through condion`
  (params (Condition :type Boolean) (`Pass through Value` :type "Float (double-precision)"))
  (returns (`Return Value` :type "Float (double-precision)"))
  (if Condition
    (return `Pass through Value`)))

(fn `Pick Up Mechanism`
  (returns (isGrabbed :type Boolean))
  (bind _hit_component_on_thunb (`self.Hit Component on thunb`))
  (bind _returnvalue (and (`self.isHit_thumb`) (`self.isHit_index`)))
  (bind _rootcomponent (`Actor.RootComponent` (`self.Hit Actor on thumb`)))
  (if (`self.IsGrabbed`)
    (if (not _returnvalue)
      (`/Engine/EditorBlueprintResources/StandardMacros.IsValid` _rootcomponent
        (:`Is Valid`
          (set `self.IsGrabbed` false)
          (`SceneComponent.K2_DetachFromComponent` _rootcomponent "KeepWorld" "KeepWorld" "KeepWorld" true)
          (if (`self.IsPhysicsON`)
            (`PrimitiveComponent.SetSimulatePhysics` _hit_component_on_thunb true)
            (`PrimitiveComponent.SetEnableGravity` _hit_component_on_thunb true)
            (set `self.tmpPhysics on` false))))))
  (if (or _returnvalue (and (`self.isHit_thumb`) (`self.isHit_middle`)) (and (`self.isHit_thumb`) (`self.isHit_ring`)) (and (`self.isHit_thumb`) (`self.IsHit_pinky`)))
    (set `self.IsGrabbed` true)
    (if (`self.IsPhysicsON`)
      (set `self.tmpPhysics on` true)
      (`PrimitiveComponent.SetSimulatePhysics` (`self.Hit Component on thunb`) true))
    (`self.K2_AttachToComponent` (`self.Hit Actor on thumb`) (`self.VR_Hand`) "None" "KeepWorld" "KeepWorld" "KeepWorld" true))
  (return (`self.IsGrabbed`)))

(fn `UserConstructionScript`)